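; A platform that stops every ball in the level when it is hit, toggling its shoot flag and disabling physics simulation.
; A DoOnce limits the hit, which also switches a dynamic material to a non-glowing hit color and marks the platform inactive.
; BeginPlay binds to each ball's shoot-end event.
; Reset fades the color back through a timeline, then restores the glow and re-arms the platform.
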(event OnComponentHit(Platform)
  (params (HitComponent :type Primitive%20Component%20Object%20Reference) (OtherActor :type Actor%20Object%20Reference) (OtherComp :type Primitive%20Component%20Object%20Reference) (NormalImpulse :type Vector :default "0, 0, 0") (Hit :type Hit%20Result%20Structure%20%28by%20ref%29))
  (bind _color (Variables|Default|GetColor))
  (Utilities|FlowControl|DoOnce false
    (:Completed
      (bind _outactors (Actor|GetAllActorsOfClass "/Game/Platformer/Blueprints/BP_Ball.BP_Ball_C"))
      (for _array_element _outactors
        (Default|CanShootBooleanChange _array_element)
        (Physics|SetSimulatePhysics (Variables|/Game/Platformer/Blueprints/BP_Ball.BP_Ball_C|GetStaticMesh _array_element) false)
        (Rendering|Material|SetVectorParameterValue _color "Color" (Variables|Default|GetHitColor) :!class /Script/Engine.MaterialInstanceDynamic)
        (Rendering|Material|SetScalarParameterValue _color "EmissiveIntensity" 0.0 :!class /Script/Engine.MaterialInstanceDynamic)
        (Variables|Default|SetbIsActive false)))))

(event Custom|Reset
  (bind _color (Variables|Default|GetColor))
  (if (not (Variables|Default|GetbIsActive))
    (Utilities|FlowControl|DoOnce false
      (:Completed
        (bind _newtrack_0 (Timeline|Timeline PlayFromStart)
          (:Update
            (Rendering|Material|SetVectorParameterValue (Variables|Default|GetColor) "Color" (Math|Color|Lerp(LinearColor) (Variables|Default|GetNotActiveColor) (Variables|Default|GetActiveColor) _newtrack_0) :!class /Script/Engine.MaterialInstanceDynamic))
          (:Finished
            (Variables|Default|SetbIsActive true)
            (CallFunction|TimelineReset)
            (Rendering|Material|SetScalarParameterValue (Variables|Default|GetColor) "EmissiveIntensity" (Variables|Default|GetEmissiveIntensity) :!class /Script/Engine.MaterialInstanceDynamic)
            (Utilities|FlowControl|DoOnce false) ; enters at Reset
          ))))))

(event Custom|TimelineReset
  (bind _color (Variables|Default|GetColor))
  (Utilities|FlowControl|DoOnce false) ; enters at Reset
)

(event EventBeginPlay
  (bind _returnvalue (Rendering|Material|CreateDynamicMaterialInstance "/Game/Platformer/Materials/M_StopPlatform.M_StopPlatform" "None" "None" :!class /Script/Engine.KismetMaterialLibrary))
  (bind _output_get (Variables|Default|SetColor _returnvalue))
  (Rendering|Material|SetVectorParameterValue _output_get "Color" (Variables|Default|GetActiveColor) :!class /Script/Engine.MaterialInstanceDynamic)
  (Rendering|Material|SetScalarParameterValue _output_get "EmissiveIntensity" (Variables|Default|GetEmissiveIntensity) :!class /Script/Engine.MaterialInstanceDynamic)
  (Rendering|Material|SetMaterial (Variables|Default|GetPlatform) 0 (Variables|Default|GetColor))
  (bind _outactors (Actor|GetAllActorsOfClass "/Game/Platformer/Blueprints/BP_Ball.BP_Ball_C"))
  (for _array_element _outactors
    (EventDispatchers|BindEventtoShootEnd _array_element (EventDispatchers|CreateEvent :!event Custom|Reset))))

(fn ConstructionScript)