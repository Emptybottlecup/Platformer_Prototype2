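; Platform that turns dangerous for a short time after the player's ball hits it.
; A hit while safe calls CanShootBooleanChange on the BP_Ball, then after a brief delay clears Active for a few seconds before restoring it.
; A hit while dangerous opens Example_Map.
; Tick sets the mesh material every frame from Active, stone when safe and red when dangerous.
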(event OnComponentHit(StaticMesh)
  (params (HitComponent :type Primitive%20Component%20Object%20Reference) (OtherActor :type Actor%20Object%20Reference) (OtherComp :type Primitive%20Component%20Object%20Reference) (NormalImpulse :type Vector :default "0, 0, 0") (Hit :type Hit%20Result%20Structure%20%28by%20ref%29))
  (if (== OtherActor (Variables|Default|GetPlayer))
    (if (Variables|Default|GetbActive)
      (Default|CanShootBooleanChange (Variables|Default|GetPlayer))
      (Utilities|FlowControl|Delay 0.2)
      (Variables|Default|SetbActive false)
      (Utilities|FlowControl|Delay 3.0)
      (Variables|Default|SetbActive true)
      (else
        (Game|OpenLevel(byName) "Example_Map")))))

(event EventBeginPlay
  (bind _asbp_ball (Utilities|Casting|CastToBP_Ball (Game|Player|GetPlayerPawn 0)))
  (Variables|Default|SetPlayer _asbp_ball))

(event EventTick
  (params (DeltaSeconds :type Float%20%28single-precision%29))
  (if (Variables|Default|GetbActive)
    (Rendering|Material|SetMaterial (Variables|Default|GetStaticMesh) 0 "/Game/Materials/Stone_Mat.Stone_Mat")
    (else
      (Rendering|Material|SetMaterial (Variables|Default|GetStaticMesh) 0 "/AnimationSharing/AnimSharingRed.AnimSharingRed"))))

(fn ConstructionScript)